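; Day-night cycle Blueprint that rotates a LightSource and refreshes the SkySphere's sun direction on Tick and in the construction script.
; Math expressions derive daylight length, yaw direction and noon height from Latitude and a 23.5-degree seasonal declination over DayCount/Year.
; Time accumulators drive yaw and separate sine pitch arcs for day and night.
; During night, Pitch exceeding Day increments DayCount, which wraps at Year, and resets PitchDrive.
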(event EventTick
  (params (DeltaSeconds :type Float%20%28single-precision%29))
  ;[1 1 1] Initialize
  (Variables|Default|SetEquatorFlip (|((((cos(((({491E5E86-4888-3FF0-FDAA-4F9E276270A8}/{342A2676-403D-072B-7E83-DA861A4A2E66})*2)*3.141590)))*23.500000)+{42C8EE59-42C5-A2D8-FF4D-0DB359398217})/(abs((((cos(((({491E5E86-4888-3FF0-FDAA-4F9E276270A8}/{342A2676-403D-072B-7E83-DA861A4A2E66})*2)*3.141590)))*23.500000)+{42C8EE59-42C5-A2D8-FF4D-0DB359398217}))))))
  (Variables|Default|SetYawDrive (+ (* DeltaSeconds (Variables|Default|GetEquatorFlip)) (Variables|Default|GetYawDrive)))
  (Variables|Default|SetPitchDrive (+ DeltaSeconds (Variables|Default|GetPitchDrive)))
  (Variables|Default|SetdayLight (|(((((arccos(((tan((({42C8EE59-42C5-A2D8-FF4D-0DB359398217}*3.141590)/180)))*(tan(((((cos(((({491E5E86-4888-3FF0-FDAA-4F9E276270A8}/{342A2676-403D-072B-7E83-DA861A4A2E66})*2)*3.141590)))*23.500000)*3.141590)/180))))))/((15*3.141590)/180))/24)*{16188202-48DD-C24D-7DF7-66A51061F2AC})*2)))
  (Variables|Default|SetNightTime (|({16188202-48DD-C24D-7DF7-66A51061F2AC}-{2FA7DC79-46AE-D34B-C7AB-BA96BDDBF9CD})))
  (if (< (Variables|Default|GetDayCount) (Variables|Default|GetYear))
    _
    (else
      (Variables|Default|SetDayCount 0.0)))
  ;[1 1 1] Day&Night  Check
  (if (< (Variables|Default|GetPitchDrive) (Variables|Default|GetdayLight))
    (Transformation|SetActorRotation (Variables|Default|GetLightSource) (Math|Rotator|MakeRotator 0.0 (|((sin(((((({7A7635A5-424E-800B-97FC-9E88A7633F92}-{2FA7DC79-46AE-D34B-C7AB-BA96BDDBF9CD})/{2FA7DC79-46AE-D34B-C7AB-BA96BDDBF9CD})/2)*2)*3.141590)))*(90-(abs((((cos(((({491E5E86-4888-3FF0-FDAA-4F9E276270A8}/{342A2676-403D-072B-7E83-DA861A4A2E66})*2)*3.141590)))*23.500000)+{42C8EE59-42C5-A2D8-FF4D-0DB359398217})))))) (|((({24B2A31D-4A86-53E0-3E72-8790D7104D24}+(({409A5541-42BE-7770-DF9A-12BB4C7D6584}*(({16188202-48DD-C24D-7DF7-66A51061F2AC}/2)-{2FA7DC79-46AE-D34B-C7AB-BA96BDDBF9CD}))/2))*360)/{16188202-48DD-C24D-7DF7-66A51061F2AC}))))
    (Default|UpdateSunDirection (Variables|Default|GetSkySphere))
    (else
      ;[1 1 1] Night
      (Transformation|SetActorRotation (Variables|Default|GetLightSource) (Math|Rotator|MakeRotator 0.0 (|((sin(((((({7A7635A5-424E-800B-97FC-9E88A7633F92}-{2FA7DC79-46AE-D34B-C7AB-BA96BDDBF9CD})/{219CA637-4D59-08A7-24DB-FBB36D7F37FC})/2)*2)*3.141590)))*90)) (|((({24B2A31D-4A86-53E0-3E72-8790D7104D24}+(({409A5541-42BE-7770-DF9A-12BB4C7D6584}*(({16188202-48DD-C24D-7DF7-66A51061F2AC}/2)-{2FA7DC79-46AE-D34B-C7AB-BA96BDDBF9CD}))/2))*360)/{16188202-48DD-C24D-7DF7-66A51061F2AC}))))
      (Default|UpdateSunDirection (Variables|Default|GetSkySphere))
      (if (> (Variables|Default|GetPitch) (Variables|Default|GetDay))
        (Variables|Default|SetDayCount (+ (Variables|Default|GetDayCount) 1.0))
        (Variables|Default|SetPitchDrive 0.0)))))

(fn ConstructionScript
  (Transformation|SetActorRotation (Variables|Default|GetLightSource) (Math|Rotator|MakeRotator 0.0 (Variables|Default|GetPitch) (Variables|Default|GetYaw)))
  (Default|UpdateSunDirection (Variables|Default|GetSkySphere)))